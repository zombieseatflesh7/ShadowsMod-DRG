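; Player character Blueprint whose graphs are mostly empty stubs, covering shield regen, selfie camera, headlight, confetti, character audio and stat updates.
; A handful of events, such as BeginPlay, possession, mesh updates, headlight-on, end-screen prep and field-medic revive effects, only forward to the parent class.
; Down-camera and Beast Master component getters return parent results, while DamageCausesReaction always returns false.
; The construction script, timeline callbacks and selfie input handlers contain no logic.
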(event `self.ReceiveBeginPlay`
  (`parent.ReceiveBeginPlay`))

(event `ShieldRegenTimeline__FinishedFunc`)

(event `ShieldRegenTimeline__UpdateFunc`)

(event `Emergency Timeline__FinishedFunc`)

(event `Emergency Timeline__UpdateFunc`)

(event `self.BP_OnControllerReady`
  (`parent.BP_OnControllerReady`))

(event `StopRegenAudio`)

(event `self.BP_OnUpdateMeshes`
  (`parent.BP_OnUpdateMeshes`))

(event `CharacterState Changed`
  (params (newState :type "ECharacterState Enum" :default "Walking")))

(event `Init Selfie Cam`)

(event `SetDustVisible`
  (params (Visible :type Boolean)))

(event `self.ReceiveOnHeadlightOn`
  (`parent.ReceiveOnHeadlightOn`))

(event `ResetSaveGameIDInEditor`)

(event `On Temporary Buff Changed`
  (params (buff :type "TemporaryBuff Object Reference") (AffectedPlayer :type "PlayerCharacter Object Reference")))

(event `MixerClientSpawnConfettii`
  (params (Location :type "Vector Structure") (Rotation :type "Rotator Structure")))

(event `MixerServerSpawnConfettii`
  (params (Location :type "Vector Structure") (Rotation :type "Rotator Structure")))

(event `MixerSpawnConfetti`
  (params (Location :type "Vector Structure") (Rotation :type "Rotator Structure")))

(event `self.PrepareForEndScreen`
  (`parent.PrepareForEndScreen`))

(event `self.Receive_ShowFieldMedicInstantReviveEffects`
  (`parent.Receive_ShowFieldMedicInstantReviveEffects`))

(event `InpAxisKeyEvt_MouseX_K2Node_InputAxisKeyEvent_0`
  (params (AxisValue :type "Float (double-precision)")))

(event `InpAxisKeyEvt_MouseY_K2Node_InputAxisKeyEvent_1`
  (params (AxisValue :type "Float (double-precision)")))

(event `SelfieZoom`
  (params (InDelta :type "Float (double-precision)")))

(event `TickSelfieZoom`)

(event `SelfieMoveUp`
  (params (InDirection :type "Float (double-precision)")))

(event `TickSelfieMoveUp`)

(event `SelfieMoveRight`
  (params (InDirection :type "Float (double-precision)")))

(event `TickSelfieMoveRight`)

(event `self.ReceivePossessed`
  (params (NewController :type "Controller Object Reference"))
  (`parent.ReceivePossessed` NewController))

(event `Cheat_Medical`)

(event `Update MissionStats`)

(fn `CharacterAudioThrottled`
  (params (Shout :type "DialogDataAsset Object Reference")))

(fn `ChromaEffect`
  (params (effect :type Byte)))

(fn `DamageCausesReaction`
  (params (DamageClass :type "DamageClass Object Reference"))
  (returns (ReturnValue :type Boolean))
  (return false))

(fn `GetBeastMasterUsableComponent`
  (returns (ReturnValue :type "UsableComponent Object Reference"))
  (return (`parent.GetBeastMasterUsableComponent`)))

(fn `GetDownCameraAttachPoint`
  (returns (ReturnValue :type "SceneComponent Object Reference"))
  (bind _returnvalue (`parent.GetDownCameraAttachPoint`))
  (return _returnvalue))

(fn `GetDownCameraRotationPoint`
  (returns (ReturnValue :type "SceneComponent Object Reference"))
  (bind _returnvalue (`parent.GetDownCameraRotationPoint`))
  (return _returnvalue))

(fn `GotoNextSelfiePoint`
  (params (ForceExitSelfieMode :type Boolean)))

(fn `SetActiveSelfiePoint`
  (params (InSelfiePoint :type "/Game/Character/Camera/BP_SelfiePoint Object Reference")))

(fn `UpdateHeadLight`)

(fn `UpdateWeaponLicenseStat`)

(fn `UserConstructionScript`)